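; Breakable potion prop that makes noise when it shatters and alerts a cat guard.
; The construction script picks one of three destructible meshes from PotEnum.
; On fracture it plays audio, switches collision to physics only, and passes its location to TriggerSoundState on the first MyCatGuard2 found in the level.
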(event `self.Destructible.OnComponentFracture`
  (params (HitPoint :type "Vector Structure (by ref)") (HitDirection :type "Vector Structure (by ref)"))
  (`AudioComponent.Play` (`self.Audio`) 0.0)
  (`PrimitiveComponent.SetCollisionEnabled` (`self.Destructible`) "PhysicsOnly")
  (bind _outactors (`GameplayStatics.GetAllActorsOfClass` "/Game/Blueprints/MyCatGuard2.MyCatGuard2_C"))
  (`CatGuard.TriggerSoundState` (`|GetArrayItem` _outactors) (`SceneComponent.K2_GetComponentLocation` (`self.Destructible`))))

(event `self.ReceiveBeginPlay`)

(fn `UserConstructionScript`
  (bind _destructible (`self.Destructible`))
  (switch `/Game/Blueprints/Enum_Potions` (`self.PotEnum`)
    (:`NewEnumerator0`
      (`DestructibleComponent.SetDestructibleMesh` _destructible "/Game/Geometry/Meshes/LevelMeshes/SM_Potion_01a_DM.SM_Potion_01a_DM"))
    (:`NewEnumerator1`
      (`DestructibleComponent.SetDestructibleMesh` _destructible "/Game/Geometry/Meshes/LevelMeshes/SM_Potion_01b_DM.SM_Potion_01b_DM"))
    (:`NewEnumerator2`
      (`DestructibleComponent.SetDestructibleMesh` _destructible "/Game/Geometry/Meshes/LevelMeshes/SM_Potion_02a_DM.SM_Potion_02a_DM"))))
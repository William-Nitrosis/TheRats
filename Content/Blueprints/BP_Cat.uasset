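; BP_Cat is an AI-driven cat that can be sent to search a location.
; StartSearch sets the Searching flag and has the cat's AI controller move it to SearchLocation, accepting a partial path.
; The construction script records the actor's position as HomeLocation, which is not read in these graphs.
; Tick branches on Searching but has no behavior yet, and BeginPlay is empty.
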(event `self.ReceiveBeginPlay`)

(event `self.ReceiveTick`
  (params (DeltaSeconds :type "Float (single-precision)"))
  (if (`self.Searching`)
    _))

(event `StartSearch`
  (set `self.Searching` true)
  (`AITask_MoveTo.AIMoveTo` (`AIBlueprintHelperLibrary.GetAIController` self) (`self.SearchLocation`) null -1.0 "Default" "Enable"))

(fn `UserConstructionScript`
  (set `self.HomeLocation` (`self.K2_GetActorLocation`)))
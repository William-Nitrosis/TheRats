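; Guard is an AI-moved Blueprint that patrols back and forth between two goal actors, Point1 and Point2.
; On BeginPlay it heads to Point2 through SimpleMoveToActor on its controller.
; Each actor overlap toggles a FlipFlop that sends it to Point1, then Point2, alternately, without checking what it overlapped.
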(event `self.ReceiveBeginPlay`
  (`NavigationSystem.SimpleMoveToActor` (`self.GetController`) (`self.Point2`)))

(event `self.ReceiveActorBeginOverlap`
  (params (OtherActor :type "Actor Object Reference"))
  (`/Engine/EditorBlueprintResources/StandardMacros.FlipFlop`
    (:`A`
      (set `self.goal` (`self.Point1`)))
    (:`B`
      (set `self.goal` (`self.Point2`))))
  (`NavigationSystem.SimpleMoveToActor` (`self.GetController`) (`self.goal`)))

(event `self.ReceiveTick`
  (params (DeltaSeconds :type "Float (single-precision)")))

(fn `UserConstructionScript`)
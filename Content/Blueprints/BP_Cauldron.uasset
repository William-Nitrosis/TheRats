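; A cauldron actor where the player drops off a carried item.
; Entering the sound sphere plays the cauldron audio, with nothing active to stop it on exit.
; Entering the drop-in area while carrying an item plays a drop sound, clears the player's carried item and pickup mesh, increments their dropped-item count, and spawns a particle effect at the glitter spawn point.
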(event `self.ReceiveBeginPlay`)

(event `self.SoundSphere.OnComponentBeginOverlap`
  (params (OverlappedComponent :type "PrimitiveComponent Object Reference") (OtherActor :type "Actor Object Reference") (OtherComp :type "PrimitiveComponent Object Reference") (OtherBodyIndex :type Integer) (bFromSweep :type Boolean) (SweepResult :type "HitResult Structure (by ref)"))
  (bind _asbp_player (cast `/Game/Blueprints/BP_player` OtherActor))
  (set `self.CharRef` _asbp_player)
  (`AudioComponent.Play` (`self.Cauldron`) 0.0))

(event `self.SoundSphere.OnComponentEndOverlap`
  (params (OverlappedComponent :type "PrimitiveComponent Object Reference") (OtherActor :type "Actor Object Reference") (OtherComp :type "PrimitiveComponent Object Reference") (OtherBodyIndex :type Integer)))

(event `self.DropInArea.OnComponentBeginOverlap`
  (params (OverlappedComponent :type "PrimitiveComponent Object Reference") (OtherActor :type "Actor Object Reference") (OtherComp :type "PrimitiveComponent Object Reference") (OtherBodyIndex :type Integer) (bFromSweep :type Boolean) (SweepResult :type "HitResult Structure (by ref)"))
  (bind _asbp_player (cast `/Game/Blueprints/BP_player` OtherActor))
  (if (`/Game/Blueprints/BP_player.CarryingItem` _asbp_player)
    (`AudioComponent.Play` (`self.DroppingInItem`) 0.0)
    (set `/Game/Blueprints/BP_player.CarryingItem` false _asbp_player)
    (`StaticMeshComponent.SetStaticMesh` (`/Game/Blueprints/BP_player.SM_pickup` _asbp_player) null)
    (`/Engine/EditorBlueprintResources/StandardMacros.IncrementInt` (`/Game/Blueprints/BP_player.ItemsDropped` _asbp_player)
      (:`  `
        (`GameplayStatics.SpawnEmitterAtLocation` "/Game/Geometry/Materials/P_Cauldron.P_Cauldron" (`SceneComponent.K2_GetComponentLocation` (`self.GlitterSpawnPoint`)))))))

(fn `UserConstructionScript`)